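; AI controller for the Scientist NPC that runs its behavior tree and supplies it with patrol and player-detection data.
; On BeginPlay it copies the pawn's patrol path looping and wait time to the blackboard, along with a patrol flag and starting direction.
; AI Perception updates for the player character write the sensed result to CanSeePlayer.
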(event `self.ReceiveBeginPlay`
  (bind _returnvalue (`AIBlueprintHelperLibrary.GetBlackboard` null))
  (bind _returnvalue_2 (`AIBlueprintHelperLibrary.GetBlackboard` null))
  (`self.RunBehaviorTree` "/Game/AI/Scientist/BT_Scientist.BT_Scientist")
  (bind _asbp_scientist (cast `/Game/AI/Scientist/BP_Scientist` (`self.K2_GetPawn`)))
  (bind _output_get (set `self.ControlledPawn` _asbp_scientist))
  (bind _patrolpath (`/Game/AI/Scientist/BP_Scientist.PatrolPath` _output_get))
  (`/Engine/EditorBlueprintResources/StandardMacros.IsValid` _patrolpath
    (:`Is Valid`
      (set `/Game/AI/Scientist/BP_Scientist.HasPatrol` true _output_get)
      (`BlackboardComponent.SetValueAsBool` _returnvalue_2 "PathLooping" (`/Game/AI/GuardNPC/PatrolPath.IsLooping` _patrolpath))
      (`BlackboardComponent.SetValueAsFloat` _returnvalue "WaitTime" (`/Game/AI/GuardNPC/PatrolPath.WaitTime` _patrolpath)))
    (:`Is Not Valid`
      (set `/Game/AI/Scientist/BP_Scientist.HasPatrol` false _output_get)))
  (`BlackboardComponent.SetValueAsBool` _returnvalue_2 "HasPatrol" (`/Game/AI/Scientist/BP_Scientist.HasPatrol` (`self.ControlledPawn`)))
  (`BlackboardComponent.SetValueAsInt` _returnvalue "Direction" 1))

(event `self.AIPerception.OnTargetPerceptionUpdated`
  (params (Actor :type "Actor Object Reference") (Stimulus :type "AIStimulus Structure"))
  (cast `/Game/Character/PlayerCharacter_BP` Actor)
  (if true
    (`BlackboardComponent.SetValueAsBool` (`AIBlueprintHelperLibrary.GetBlackboard` null) "CanSeePlayer" Stimulus_bSuccessfullySensed)))

(fn `UserConstructionScript`)