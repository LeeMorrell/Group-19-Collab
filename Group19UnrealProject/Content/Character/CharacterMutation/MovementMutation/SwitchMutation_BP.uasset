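; SwitchMutation_BP is a movement mutation that swaps the player's position with a pawn in front of them.
; On activation, it runs a Visibility line trace from the parent player character's ForwardArrow out to SwitchRange, kept at arrow height, with debug drawing on.
; If a pawn is hit, the player teleports to the pawn's location and the pawn to the arrow's saved location.
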(event `/Game/Character/CharacterMutation/MutationInterface.ActivateMovementMutation`
  (bind _asplayer_character_bp (cast `/Game/Character/PlayerCharacter_BP` (`self.GetParentActor`)))
  (bind _forwardarrow (`/Game/Character/PlayerCharacter_BP.ForwardArrow` _asplayer_character_bp))
  (bind (_returnvalue_x _returnvalue_y _returnvalue_z) (`KismetMathLibrary.BreakVector` (`SceneComponent.K2_GetComponentLocation` _forwardarrow)))
  (bind _output_get (set `self.PCLocation` (`KismetMathLibrary.MakeVector` _returnvalue_x _returnvalue_y _returnvalue_z)))
  (bind (_returnvalue_x_2 _returnvalue_y_2) (`KismetMathLibrary.BreakVector` (+ (`KismetMathLibrary.MakeVector` _returnvalue_x _returnvalue_y _returnvalue_z) (* (`SceneComponent.GetForwardVector` _forwardarrow) (`self.SwitchRange`)))))
  (bind (_outhit _returnvalue) (`KismetSystemLibrary.LineTraceSingle` _output_get (`KismetMathLibrary.MakeVector` _returnvalue_x_2 _returnvalue_y_2 _returnvalue_z) "TraceTypeQuery1" false (`|MakeArray` (`GameplayStatics.GetPlayerCharacter` 0) :!type "Actor Object Reference") "ForDuration" true (struct :`R` 1.0 :`A` 1.0) (struct :`G` 1.0 :`A` 1.0) 1.0))
  (if _returnvalue
    (bind _aspawn (cast `Pawn` (`.HitActor` (`GameplayStatics.BreakHitResult` _outhit))))
    (bind _output_get_2 (set `self.EnemyLocation` (`self.K2_GetActorLocation` _aspawn)))
    (`self.K2_SetActorLocation` (`self.GetParentActor`) _output_get_2 false true)
    (`self.K2_SetActorLocation` _aspawn (`self.PCLocation`) false true)))

(fn `UserConstructionScript`
  (`parent.UserConstructionScript`))