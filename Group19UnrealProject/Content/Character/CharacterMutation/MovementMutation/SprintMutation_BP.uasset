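; Sprint movement mutation actor that gives its parent player character a temporary walk speed boost.
; On activation it saves the current MaxWalkSpeed, adds the sprint increase and attaches a sprint particle emitter to the character mesh.
; A one-shot timer then restores the saved speed and destroys the emitter.
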(event `/Game/Character/CharacterMutation/MutationInterface.ActivateMovementMutation`
  (bind _asplayer_character_bp (cast `/Game/Character/PlayerCharacter_BP` (`self.GetParentActor`)))
  (bind _charactermovement (`Character.CharacterMovement` _asplayer_character_bp))
  (bind _maxwalkspeed (`CharacterMovementComponent.MaxWalkSpeed` _charactermovement))
  (set `self.BaselineMovementSpeed` _maxwalkspeed)
  (set `CharacterMovementComponent.MaxWalkSpeed` (+ _maxwalkspeed (`self.SprintMoveIncrease`)) _charactermovement)
  (bind _mesh (`Character.Mesh` _asplayer_character_bp))
  (bind (_returnvalue_x _returnvalue_y) (`KismetMathLibrary.BreakVector` (`SceneComponent.GetForwardVector` _mesh)))
  (bind _returnvalue (`GameplayStatics.SpawnEmitterAttached` "/Game/Particles/Sprint/P_Sprint.P_Sprint" _mesh "None" (0.0 0.0 0.0) (`KismetMathLibrary.MakeRotator` _returnvalue_x _returnvalue_y 270.0)))
  (`KismetSystemLibrary.K2_SetTimerDelegate` (delegate `ResetSpeed`) (`self.SprintTime`)))

(event `ResetSpeed`
  (set `CharacterMovementComponent.MaxWalkSpeed` (`self.BaselineMovementSpeed`) (`Character.CharacterMovement` (stale `/Game/Character/CharacterMutation/MutationInterface.ActivateMovementMutation` _asplayer_character_bp)))
  (`ActorComponent.K2_DestroyComponent` (stale `/Game/Character/CharacterMutation/MutationInterface.ActivateMovementMutation` _returnvalue)))

(fn `UserConstructionScript`
  (`parent.UserConstructionScript`))