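; Blueprint for a vampiric attack mutation, an extra character mutation that trades attack damage for health.
; On extra-mutation activation it casts its parent actor to PlayerCharacter_BP and adds its attack damage reduction to that character's outgoing damage reduction.
; On attack-mutation activation it sends the parent actor a health change message carrying the vampiric health increase.
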(event `/Game/Character/CharacterMutation/MutationInterface.ActivateExtraMutation`
  (bind _asplayer_character_bp (cast `/Game/Character/PlayerCharacter_BP` (`self.GetParentActor`)))
  (set `/Game/Character/PlayerCharacter_BP.OutgoingDamageReduction` (+ (`/Game/Character/PlayerCharacter_BP.OutgoingDamageReduction` _asplayer_character_bp) (`self.AttackDamageReduction`)) _asplayer_character_bp))

(event `/Game/Character/CharacterMutation/MutationInterface.ActivateAttackMutation`
  (params (OutgoingDamageReduction :type "Float (single-precision)"))
  (message `/Game/Character/CharacterMutation/MutationInterface.ChangeCharacterHealth` (`self.GetParentActor`) (`self.VampiricHealthIncrease`)))

(fn `UserConstructionScript`
  (`parent.UserConstructionScript`))