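; Base Blueprint for extra mutations that change player stats, acting on the parent actor when it is a PlayerCharacter_BP.
; ActivateExtraMutation adds each non-zero modifier to the player's attack, damage reduction, movement or health stats.
; The movement cooldown branch checks NewMoveMutationCooldown but adds NewMovementSpeed, so the cooldown value itself is never applied.
; The changes are plain additions with no removal logic.
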(event `/Game/Character/CharacterMutation/MutationInterface.ActivateExtraMutation`
  (bind _asplayer_character_bp (cast `/Game/Character/PlayerCharacter_BP` (`self.GetParentActor`)))
  (if (!= (`self.NewAttackSpeed`) 0.0)
    (set `/Game/Character/PlayerCharacter_BP.RateOfAttack` (+ (`/Game/Character/PlayerCharacter_BP.RateOfAttack` _asplayer_character_bp) (`self.NewAttackSpeed`)) _asplayer_character_bp))
  (if (!= (`self.NewAttackDamageReduction`) 0.0)
    (set `/Game/Character/PlayerCharacter_BP.OutgoingDamageReduction` (+ (`/Game/Character/PlayerCharacter_BP.OutgoingDamageReduction` _asplayer_character_bp) (`self.NewAttackDamageReduction`)) _asplayer_character_bp))
  (if (!= (`self.NewMoveMutationCooldown`) 0.0)
    (set `/Game/Character/PlayerCharacter_BP.MovementCooldown` (+ (`/Game/Character/PlayerCharacter_BP.MovementCooldown` _asplayer_character_bp) (`self.NewMovementSpeed`)) _asplayer_character_bp))
  (if (!= (`self.NewMovementSpeed`) 0.0)
    (bind _charactermovement (`Character.CharacterMovement` _asplayer_character_bp))
    (set `CharacterMovementComponent.MaxWalkSpeed` (+ (`CharacterMovementComponent.MaxWalkSpeed` _charactermovement) (`self.NewMovementSpeed`)) _charactermovement))
  (if (!= (`self.NewMaxHealth`) 0.0)
    (set `/Game/Character/PlayerCharacter_BP.MaxHealth` (+ (`/Game/Character/PlayerCharacter_BP.MaxHealth` _asplayer_character_bp) (`self.NewMaxHealth`)) _asplayer_character_bp))
  (if (!= (`self.NewIncomingDamageReduction`) 0.0)
    (set `/Game/Character/PlayerCharacter_BP.IncomingDamageReduction` (+ (`/Game/Character/PlayerCharacter_BP.IncomingDamageReduction` _asplayer_character_bp) (`self.NewIncomingDamageReduction`)) _asplayer_character_bp)))

(fn `UserConstructionScript`
  (`parent.UserConstructionScript`))