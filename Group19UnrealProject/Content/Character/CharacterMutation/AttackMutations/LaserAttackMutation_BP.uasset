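; Attack mutation actor that fires a piercing laser from its parent player character.
; On activation it divides baseline damage by the outgoing damage reduction, then multi-line traces on Visibility from the character's forward arrow at constant height.
; It spawns the laser particle at the arrow and damages each overlapped actor until the first blocking hit, which takes no damage.
; BeginPlay caches player 0 and its child actors as trace ignores.
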(event `/Game/Character/CharacterMutation/MutationInterface.ActivateAttackMutation`
  (params (OutgoingDamageReduction :type "Float (single-precision)"))
  (set `self.Damage` (/ (`self.BaselineDamage`) OutgoingDamageReduction))
  (bind _asplayer_character_bp (cast `/Game/Character/PlayerCharacter_BP` (`self.GetParentActor`)))
  (bind _forwardarrow (`/Game/Character/PlayerCharacter_BP.ForwardArrow` _asplayer_character_bp))
  (bind (_returnvalue_x _returnvalue_y _returnvalue_z) (`KismetMathLibrary.BreakVector` (`SceneComponent.K2_GetComponentLocation` _forwardarrow)))
  (bind _returnvalue (`KismetMathLibrary.MakeVector` _returnvalue_x _returnvalue_y _returnvalue_z))
  (bind (_returnvalue_x_2 _returnvalue_y_2) (`KismetMathLibrary.BreakVector` (+ (`KismetMathLibrary.MakeVector` _returnvalue_x _returnvalue_y _returnvalue_z) (* (`SceneComponent.GetForwardVector` _forwardarrow) (`self.LaserBeamRange`)))))
  (bind _outhits (`KismetSystemLibrary.LineTraceMulti` _returnvalue (`KismetMathLibrary.MakeVector` _returnvalue_x_2 _returnvalue_y_2 _returnvalue_z) "TraceTypeQuery1" false (`self.IgnoreActors`) "ForDuration" true (struct :`R` 1.0 :`A` 1.0) (struct :`G` 1.0 :`A` 1.0) 0.0))
  (`GameplayStatics.SpawnEmitterAtLocation` "/Game/Particles/Laser/P_Laser.P_Laser" _returnvalue (`SceneComponent.K2_GetComponentRotation` _forwardarrow))
  (for _array_element _outhits
    (bind (_bblockinghit _binitialoverlap _time _distance _location _impactpoint _normal _impactnormal _physmat _hitactor) (`GameplayStatics.BreakHitResult` _array_element))
    (if _bblockinghit
      (break)
      (else
        (`GameplayStatics.ApplyDamage` _hitactor (`self.Damage`))))))

(event `self.ReceiveBeginPlay`
  (bind _returnvalue (`GameplayStatics.GetPlayerCharacter` 0))
  (bind _output_get (set `self.IgnoreActors` (`self.GetAllChildActors` _returnvalue true)))
  (`KismetArrayLibrary.Array_Add` _output_get _returnvalue))

(fn `UserConstructionScript`
  (`parent.UserConstructionScript`))