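; Lightning attack mutation, attached as a child actor of PlayerCharacter_BP, that fires a lightning bolt when activated.
; It spawns a short-lived lightning emitter at the player's ForwardArrow and multi-traces on Visibility along it at constant height, ignoring the player.
; Only the first hit takes direct damage.
; Full-strength radial burst damage is centred on that hit's TraceEnd, the far end of the trace rather than the impact point.
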(event `/Game/Character/CharacterMutation/MutationInterface.ActivateAttackMutation`
  (params (OutgoingDamageReduction :type "Float (single-precision)"))
  (bind _asplayer_character_bp (cast `/Game/Character/PlayerCharacter_BP` (`self.GetParentActor`)))
  (`KismetArrayLibrary.Array_AddUnique` (`self.Ignore`) _asplayer_character_bp)
  (bind _forwardarrow (`/Game/Character/PlayerCharacter_BP.ForwardArrow` _asplayer_character_bp))
  (bind _returnvalue (`GameplayStatics.SpawnEmitterAtLocation` "/Game/Particles/Lightning/P_lightning.P_lightning" (`SceneComponent.K2_GetComponentLocation` _forwardarrow) (`SceneComponent.K2_GetComponentRotation` _forwardarrow)))
  (bind (_returnvalue_x _returnvalue_y _returnvalue_z) (`KismetMathLibrary.BreakVector` (`SceneComponent.K2_GetComponentLocation` _forwardarrow)))
  (bind (_returnvalue_x_2 _returnvalue_y_2) (`KismetMathLibrary.BreakVector` (+ (`KismetMathLibrary.MakeVector` _returnvalue_x _returnvalue_y _returnvalue_z) (* (`SceneComponent.GetForwardVector` _forwardarrow) (`self.LightningLength`)))))
  (bind _outhits (`KismetSystemLibrary.LineTraceMulti` (`KismetMathLibrary.MakeVector` _returnvalue_x _returnvalue_y _returnvalue_z) (`KismetMathLibrary.MakeVector` _returnvalue_x_2 _returnvalue_y_2 _returnvalue_z) "TraceTypeQuery1" false (`self.Ignore`) "None" true (struct :`R` 1.0 :`A` 1.0) (struct :`G` 1.0 :`A` 1.0) 0.0))
  (bind (_output_bblockinghit _output_binitialoverlap _output_time _output_distance _output_location _output_impactpoint _output_normal _output_impactnormal _output_physmat _output_hitactor _output_hitcomponent _output_hitbonename _output_hititem _output_faceindex _output_tracestart _output_traceend) (`GameplayStatics.BreakHitResult` (`|GetArrayItem` _outhits)))
  (`GameplayStatics.ApplyDamage` _output_hitactor (`self.Damage`) (`GameplayStatics.GetPlayerController` 0) self)
  (`GameplayStatics.ApplyRadialDamage` (`self.BurstDamage`) _output_traceend 100.0 null (`self.Ignore`) null null true)
  (`KismetSystemLibrary.Delay` 0.2)
  (`ActorComponent.K2_DestroyComponent` _returnvalue))

(fn `UserConstructionScript`
  (`parent.UserConstructionScript`))