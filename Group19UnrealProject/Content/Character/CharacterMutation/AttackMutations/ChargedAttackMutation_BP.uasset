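; Charged attack mutation Blueprint that delays a character's mutated attack by a charge time.
; It overrides ActivateAttackMutation to start a one-shot timer behind a DoOnce, so repeat activations during the charge are ignored.
; When the timer fires, the Attack event calls the parent activation with the outgoing damage reduction and resets the DoOnce.
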(event `/Game/Character/CharacterMutation/MutationInterface.ActivateAttackMutation`
  (params (OutgoingDamageReduction :type "Float (single-precision)"))
  (`/Engine/EditorBlueprintResources/StandardMacros.DoOnce` false :!label _label
    (:`Completed`
      (`KismetSystemLibrary.K2_SetTimerDelegate` (delegate `Attack`) (`self.ChargeTime`)))))

(event `Attack`
  (`parent.ActivateAttackMutation` (stale `/Game/Character/CharacterMutation/MutationInterface.ActivateAttackMutation` OutgoingDamageReduction))
  (goto _label :!via `Reset`))

(fn `UserConstructionScript`
  (`parent.UserConstructionScript`))