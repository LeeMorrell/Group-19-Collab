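; Bomb actor for an automatic-bomb attack mutation that explodes on a timer.
; BeginPlay starts a one-shot timer that applies full radial damage at the bomb's location, ignoring the first player's character, then destroys the actor.
; ActivateAttackMutation divides the bomb's damage by a supplied outgoing damage reduction factor.
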(event `self.ReceiveBeginPlay`
  (`KismetSystemLibrary.K2_SetTimerDelegate` (delegate `Explosion`) (`self.BombTimer`)))

(event `Explosion`
  (`GameplayStatics.ApplyRadialDamage` (`self.Damage`) (`self.K2_GetActorLocation`) (`self.ExplosionRadius`) null (`|MakeArray` (`GameplayStatics.GetPlayerCharacter` 0) :!type "Actor Object Reference") null null true)
  (`self.K2_DestroyActor`))

(event `/Game/Character/CharacterMutation/MutationInterface.ActivateAttackMutation`
  (params (OutgoingDamageReduction :type "Float (single-precision)"))
  (set `self.Damage` (/ (`self.Damage`) OutgoingDamageReduction)))

(fn `UserConstructionScript`)