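; Ranged attack mutation actor for the player character that fires a projectile when the attack is activated.
; On activation it casts its parent actor to the player character and spawns the configured projectile class at that character's forward arrow, with the player as owner and instigator.
; It then passes the outgoing damage reduction to the new projectile through an activation message.
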(event `/Game/Character/CharacterMutation/MutationInterface.ActivateAttackMutation`
  (params (OutgoingDamageReduction :type "Float (single-precision)"))
  (bind _asplayer_character_bp (cast `/Game/Character/PlayerCharacter_BP` (`self.GetParentActor`)))
  (bind _returnvalue (`|SpawnActorFromClass` (`self.ProjectileClass`) (`SceneComponent.K2_GetComponentToWorld` (`/Game/Character/PlayerCharacter_BP.ForwardArrow` _asplayer_character_bp)) "Undefined" "OverrideRootScale" _asplayer_character_bp _asplayer_character_bp))
  (message `/Game/Character/CharacterMutation/MutationInterface.ActivateAttackMutation` _returnvalue OutgoingDamageReduction))

(fn `UserConstructionScript`
  (`parent.UserConstructionScript`))