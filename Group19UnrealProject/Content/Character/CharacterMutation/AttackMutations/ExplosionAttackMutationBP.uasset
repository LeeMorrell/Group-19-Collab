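; Attack mutation actor that gives its parent player character an explosion ability dealing full radial damage without falloff.
; On activation it freezes movement, spawns an explosion emitter at the forward arrow and applies damage at a point offset along world X.
; A short delay then restores walking.
; The player is added to an Ignore list, but that list is not wired into the damage call.
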(event `/Game/Character/CharacterMutation/MutationInterface.ActivateAttackMutation`
  (params (OutgoingDamageReduction :type "Float (single-precision)"))
  (bind _asplayer_character_bp (cast `/Game/Character/PlayerCharacter_BP` (`self.GetParentActor`)))
  (`KismetArrayLibrary.Array_AddUnique` (`self.Ignore`) _asplayer_character_bp)
  (bind _charactermovement (`Character.CharacterMovement` _asplayer_character_bp))
  (`CharacterMovementComponent.DisableMovement` _charactermovement)
  (bind (_returnvalue_x _returnvalue_y _returnvalue_z) (`KismetMathLibrary.BreakVector` (`SceneComponent.K2_GetComponentLocation` (`/Game/Character/PlayerCharacter_BP.ForwardArrow` _asplayer_character_bp))))
  (`GameplayStatics.SpawnEmitterAtLocation` "/Game/Particles/Explosion/P_ExplosionAbility.P_ExplosionAbility" (`KismetMathLibrary.MakeVector` _returnvalue_x _returnvalue_y _returnvalue_z) (struct) (2.0 2.0 2.0))
  (`GameplayStatics.ApplyRadialDamage` :`BaseDamage` (`self.Damage`) :`Origin` (`KismetMathLibrary.MakeVector` (+ _returnvalue_x 90.0) _returnvalue_y _returnvalue_z) :`DamageRadius` 500.0 :`DamageCauser` (`Controller.K2_GetPawn` (`GameplayStatics.GetPlayerController` 0)) :`InstigatedByController` null :`bDoFullDamage` true)
  (`KismetSystemLibrary.Delay` 0.4)
  (`CharacterMovementComponent.SetMovementMode` _charactermovement "MOVE_Walking" 0))

(fn `UserConstructionScript`
  (`parent.UserConstructionScript`))