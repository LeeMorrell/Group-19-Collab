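; RngAtkProjectile_BP is a projectile for the character's ranged attack mutation that damages what it hits.
; A timer started on BeginPlay destroys it after LifeSpan.
; Its Sphere overlap applies Damage and destroys the projectile, ignoring the player character and actors of its own class.
; The ActivateAttackMutation event divides Damage by the OutgoingDamageReduction passed in.
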(event `self.ReceiveBeginPlay`
  (`KismetSystemLibrary.K2_SetTimerDelegate` (delegate `Death`) (`self.LifeSpan`)))

(event `Death`
  (`self.K2_DestroyActor`))

(event `self.Sphere.OnComponentBeginOverlap`
  (params (OverlappedComponent :type "PrimitiveComponent Object Reference") (OtherActor :type "Actor Object Reference") (OtherComp :type "PrimitiveComponent Object Reference") (OtherBodyIndex :type Integer) (bFromSweep :type Boolean) (SweepResult :type "HitResult Structure (by ref)"))
  (if (and (!= (`GameplayStatics.GetPlayerCharacter` 0) OtherActor) (!= (`GameplayStatics.GetObjectClass` OtherActor) (`GameplayStatics.GetObjectClass` self)))
    (`GameplayStatics.ApplyDamage` OtherActor (`self.Damage`))
    (`self.K2_DestroyActor`)))

(event `/Game/Character/CharacterMutation/MutationInterface.ActivateAttackMutation`
  (params (OutgoingDamageReduction :type "Float (single-precision)"))
  (set `self.Damage` (/ (`self.Damage`) OutgoingDamageReduction)))

(fn `UserConstructionScript`)